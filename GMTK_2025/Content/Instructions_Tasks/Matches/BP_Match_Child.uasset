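; BP_Match_Child is a single flippable tile in a pair-matching task, owned by BP_Match_Instruction and showing its icon through a WBP_Match_Icon widget.
; A timeline rotates the mesh to reveal it, then reports its match type to the owner, and reverses to hide it.
; Player flips are blocked during solution display or when two tiles are turned.
; It also handles reset, full hiding and an overlay-material outline.
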(event `Initialise Match Child`
  (params (`Match Child Info` :type "/Game/Instructions_Tasks/Matches/Struct_Match_Child_Info Structure"))
  (bind _aswbp_match_icon (cast `/Game/UI/In-Game/WBP_Match_Icon` (`WidgetComponent.GetWidget` (`self.Match Icon`))))
  (`/Game/UI/In-Game/WBP_Match_Icon.Update Match Icon` _aswbp_match_icon `Match Child Info`)
  (`SceneComponent.K2_SetRelativeRotation` :`self` (`self.Match Child Mesh`))
  (bind _asbp_match_instruction (cast `/Game/Instructions_Tasks/Matches/BP_Match_Instruction` (`self.GetOwner`)))
  (set `self.As BP Match Instruction` _asbp_match_instruction)
  (set `self.Match Type` (`.MatchChildValue_2_D2BA696D4B564E0BC47E26BD0B8C7BA8` (break `/Game/Instructions_Tasks/Matches/Struct_Match_Child_Info` `Match Child Info`))))

(event `Show Match Child`
  (params (`IsPlayer?` :type Boolean))
  (if `IsPlayer?`
    (if (`/Game/Instructions_Tasks/Matches/BP_Match_Instruction.Solution Being Shown` (`self.As BP Match Instruction`))
      _
      (elif (or (`self.Shown`) (`TimelineComponent.IsPlaying` (`self.Visibility Match Child Timeline`)))
        _
        (elif (not (== (`/Game/Instructions_Tasks/Matches/BP_Match_Instruction.Turned Children Count` (`self.As BP Match Instruction`)) 2))
          (`FMODBlueprintStatics.PlayEventAtLocation` "/Game/FMOD/Events/In-Game/Match_Show.Match_Show" (`KismetMathLibrary.MakeTransform` (`self.K2_GetActorLocation`)) :!label _label)
          (bind (_direction _alpha) (`Timeline|Visibility Match Child Timeline` :!via `PlayFromStart` :!label _label_2)
            (:`Update`
              (`SceneComponent.K2_SetRelativeRotation` (`self.Match Child Mesh`) (`KismetMathLibrary.RLerp` (struct) (struct :`Yaw` 180.0) _alpha) false false))
            (:`Finished`
              (bind _output_get (set `self.Shown` (> _alpha 0.0)))
              (if _output_get
                (`/Game/Instructions_Tasks/Matches/BP_Match_Instruction.Match Child Turned` (`self.As BP Match Instruction`) (`self.Match Type`))))))))
    (else
      (goto _label))))

(event `Hide Match Child`
  (set `self.Shown` false)
  (if (not (`TimelineComponent.IsPlaying` (`self.Visibility Match Child Timeline`)))
    (`FMODBlueprintStatics.PlayEventAtLocation` "/Game/FMOD/Events/In-Game/Match_Hide.Match_Hide" (`KismetMathLibrary.MakeTransform` (`self.K2_GetActorLocation`)))
    (goto _label_2 :!via `Reverse`)))

(event `Reset Match Child`
  (set `self.Shown` false)
  (`SceneComponent.K2_SetRelativeRotation` :`self` (`self.Match Child Mesh`))
  (`self.SetActorHiddenInGame` false))

(event `Full Hide Match Child`
  (set `self.Shown` false)
  (`SceneComponent.K2_SetRelativeRotation` :`self` (`self.Match Child Mesh`))
  (`self.SetActorHiddenInGame` true))

(event `Deactivate_Outline_1`
  (`MeshComponent.SetOverlayMaterial` (`self.Match Child Mesh`) null))

(event `Activate_Outline_1`
  (`MeshComponent.SetOverlayMaterial` (`self.Match Child Mesh`) "/Game/Assets/M_Outline.M_Outline"))

(fn `UserConstructionScript`)