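; BP_Jump_Instruction is a tutorial instruction task that completes when the player jumps.
; On setup it casts the player character to BP_Player and binds to its JumpED event dispatcher.
; A jump while the instruction is active sets a done flag, prints a debug string and calls InstructionInteract once.
; Enabling the instruction resets that flag, building on parent instruction logic for setup and enabling.
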(fn `Enable Instruction`
  (`parent.Enable Instruction`)
  (set `self.Jump Instruction Done` false))

(fn `Player Jumped`
  (if (`self.Active`)
    (if (not (`self.Jump Instruction Done`))
      (set `self.Jump Instruction Done` true)
      (`KismetSystemLibrary.PrintString` "Player Jumped Whilst active")
      (`self.Instruction Interact` true))))

(fn `Setup Instruction`
  (params (`Instruction Info` :type "/Game/Instructions_Tasks/Struct_Instruction_Info Structure"))
  (`parent.Setup Instruction` `Instruction Info`)
  (bind _asbp_player (cast `/Game/Player/Blueprints/BP_Player` (`GameplayStatics.GetPlayerCharacter` 0)))
  (add `/Game/Player/Blueprints/BP_Player.Jump ED` _asbp_player (`|CreateDelegate` :!event `Player Jumped`)))

(fn `UserConstructionScript`
  (`parent.UserConstructionScript`))