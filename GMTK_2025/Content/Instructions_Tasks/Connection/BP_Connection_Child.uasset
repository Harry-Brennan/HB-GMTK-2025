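; BP_Connection_Child is a pressable piece of the connection task, owned by a parent BP_Connection_Instruction actor.
; A press plays sound and camera shake, lowers the upper mesh on a timeline, then notifies the parent.
; Player presses are blocked while the solution is shown, but non-player presses still go through.
; Confirm and reset events set the state and material, and outline events toggle an overlay material.
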(event `self.ReceiveBeginPlay`
  (bind _asbp_connection_instruction (cast `/Game/Instructions_Tasks/Connection/BP_Connection_Instruction` (`self.GetParentActor`)))
  (set `self.As BP Connection Instruction` _asbp_connection_instruction))

(event `Press Connection Child`
  (params (`IsPlayer?` :type Boolean))
  (if `IsPlayer?`
    (if (not (`/Game/Instructions_Tasks/Connection/BP_Connection_Instruction.Solution Being Shown` (`self.As BP Connection Instruction`)))
      (if (`self.Confirmed?`) :!label _label
        _
        (elif (not (`self.Selected?`))
          (set `self.Selected?` true)
          (`FMODBlueprintStatics.PlayEventAtLocation` "/Game/FMOD/Events/In-Game/Object_Pressed.Object_Pressed" (`KismetMathLibrary.MakeTransform` (`self.K2_GetActorLocation`)))
          (`LegacyCameraShake.StartLegacyCameraShake` (`GameplayStatics.GetPlayerCameraManager` 0) "/Game/Instructions_Tasks/BP_Object_Pressed_CS.BP_Object_Pressed_CS_C")
          (bind (_direction _alpha) (`Timeline|Press Connection Child Timeline` :!via `PlayFromStart` :!label _label_2)
            (:`Update`
              (`SceneComponent.K2_SetRelativeLocation` (`self.Upper`) (`KismetMathLibrary.VLerp` (0.0 0.0 0.0) (0.0 0.0 -10.0) _alpha) false false))
            (:`Change Material`
              (`PrimitiveComponent.SetMaterial` (`self.Upper`) 0 "/Game/Assets/Interactions/M_Connection_Pressed.M_Connection_Pressed")
              (`KismetSystemLibrary.Delay` 0.05)
              (`/Game/Instructions_Tasks/Connection/BP_Connection_Instruction.Connection Child Pressed` (`self.As BP Connection Instruction`) self))))))
    (else
      (goto _label))))

(event `Confirm Connection Child`
  (set `self.Confirmed?` true)
  (`PrimitiveComponent.SetMaterial` (`self.Upper`) 0 "/Game/Assets/Interactions/M_Connection_Active.M_Connection_Active")
  (set `self.Selected?` false))

(event `Reset Connection Child`
  (bind _upper (`self.Upper`))
  (`KismetSystemLibrary.PrintString` "Reset Connection Child")
  (`|ExecutionSequence`
    (:`then_0`
      (goto _label_2 :!via `Stop`))
    (:`then_1`
      (`PrimitiveComponent.SetMaterial` _upper 0 "/Game/Assets/Interactions/M_Connection_Inactive.M_Connection_Inactive")
      (`SceneComponent.K2_SetRelativeLocation` _upper (0.0 0.0 0.0) false false)
      (`KismetSystemLibrary.Delay` 0.2)
      (set `self.Confirmed?` false)
      (set `self.Selected?` false))))

(event `Deactivate_Outline_1`
  (`MeshComponent.SetOverlayMaterial` (`self.Upper`) null)
  (`MeshComponent.SetOverlayMaterial` (`self.Lower`) null))

(event `Activate_Outline_1`
  (`MeshComponent.SetOverlayMaterial` (`self.Upper`) "/Game/Assets/M_Outline.M_Outline")
  (`MeshComponent.SetOverlayMaterial` (`self.Lower`) "/Game/Assets/M_Outline.M_Outline"))

(fn `UserConstructionScript`)