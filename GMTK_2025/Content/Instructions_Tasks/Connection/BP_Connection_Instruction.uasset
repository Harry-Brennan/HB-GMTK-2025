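; Connection instruction task where the player matches three left BP_Connection_Child actors to three right ones by hidden value.
; Setup randomly pairs the children by removing picks from both arrays, then refills them.
; First show auto-presses each pair as a demonstration, then resets them and starts the countdown and HUD timer.
; Correct pairs confirm and complete the task once all match; mismatches reset the pair and cost a life.
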(event `Initialise Left and Right Children`
  (for _index (range 3)
    (bind _asbp_connection_child (cast `/Game/Instructions_Tasks/Connection/BP_Connection_Child` (`ChildActorComponent.ChildActor` (select `int` _index :`0` (`self.Connection Child L1`) :`1` (`self.Connection Child L2`) :`2` (`self.Connection Child L3`)))))
    (`KismetArrayLibrary.Array_Add` (`self.Left Children`) _asbp_connection_child))
  (for _index_2 (range 3)
    (bind _asbp_connection_child_2 (cast `/Game/Instructions_Tasks/Connection/BP_Connection_Child` (`ChildActorComponent.ChildActor` (select `int` _index_2 :`0` (`self.Connection Child R1`) :`1` (`self.Connection Child R2`) :`2` (`self.Connection Child R3`)))))
    (`KismetArrayLibrary.Array_Add` (`self.Right Children`) _asbp_connection_child_2))
  (`/Engine/EditorBlueprintResources/StandardMacros.DoOnce` false
    (:`Completed`
      (for _index_3 (range 3)
        (bind _output_get (set `self.Current Random Left` (`KismetArrayLibrary.Array_Random` (`self.Left Children`))))
        (set `/Game/Instructions_Tasks/Connection/BP_Connection_Child.Value` _index_3 _output_get)
        (bind _output_get_2 (set `self.Current Random Right` (`KismetArrayLibrary.Array_Random` (`self.Right Children`))))
        (set `/Game/Instructions_Tasks/Connection/BP_Connection_Child.Value` _index_3 _output_get_2)
        (`KismetArrayLibrary.Array_RemoveItem` (`self.Left Children`) (`self.Current Random Left`))
        (`KismetArrayLibrary.Array_RemoveItem` (`self.Right Children`) (`self.Current Random Right`)))
      (`self.Initialise Left and Right Children`))))

(event `Connection Child Pressed`
  (params (`Child Ref` :type "/Game/Instructions_Tasks/Connection/BP_Connection_Child Object Reference"))
  (`/Engine/EditorBlueprintResources/StandardMacros.IsValid` (`self.Currently Selected Child`)
    (:`Is Valid`
      (if (== (`/Game/Instructions_Tasks/Connection/BP_Connection_Child.Value` `Child Ref`) (`/Game/Instructions_Tasks/Connection/BP_Connection_Child.Value` (`self.Currently Selected Child`)))
        (`/Game/Instructions_Tasks/Connection/BP_Connection_Child.Confirm Connection Child` (`self.Currently Selected Child`))
        (`/Game/Instructions_Tasks/Connection/BP_Connection_Child.Confirm Connection Child` `Child Ref`)
        (`FMODBlueprintStatics.PlayEventAtLocation` "/Game/FMOD/Events/In-Game/Connection_Correct.Connection_Correct" (`KismetMathLibrary.MakeTransform` (`self.K2_GetActorLocation`)))
        (set `self.Currently Selected Child` null)
        (if (not (`self.Solution Being Shown`))
          (set `self.All Children Confirmed?` true)
          (for _index (range 3)
            (if (not (`/Game/Instructions_Tasks/Connection/BP_Connection_Child.Confirmed?` (`|GetArrayItem` (`self.Left Children`) _index)))
              (set `self.All Children Confirmed?` false :!label _label)))
          (for _index_2 (range 3)
            (if (not (`/Game/Instructions_Tasks/Connection/BP_Connection_Child.Confirmed?` (`|GetArrayItem` (`self.Right Children`) _index_2)))
              (goto _label)))
          (if (`self.All Children Confirmed?`)
            (`self.Instruction Interact` true)))
        (else
          (`FMODBlueprintStatics.PlayEventAtLocation` "/Game/FMOD/Events/In-Game/Connection_Incorrect.Connection_Incorrect" (`KismetMathLibrary.MakeTransform` (`self.K2_GetActorLocation`)))
          (`/Game/Instructions_Tasks/Connection/BP_Connection_Child.Reset Connection Child` (`self.Currently Selected Child`))
          (`/Game/Instructions_Tasks/Connection/BP_Connection_Child.Reset Connection Child` `Child Ref`)
          (set `self.Currently Selected Child` null)
          (bind _asbp_player (cast `/Game/Player/Blueprints/BP_Player` (`GameplayStatics.GetPlayerCharacter` 0)))
          (`/Game/Player/Blueprints/BP_Player.Decrease Life` _asbp_player))))
    (:`Is Not Valid`
      (set `self.Currently Selected Child` `Child Ref`))))

(event `Show Connection Solution`
  (bind ((`InstructionType_2_6A9FB7814C2D0346CFAC84934FEBBF4F` _instructiontype) (`InstructionTime_32_0CE54A424D1941F04ADBD48A30216293` _instructiontime)) (break `/Game/Instructions_Tasks/Struct_Instruction_Info` (`self.Instruction Info`)))
  (set `self.Solution Being Shown` true)
  (`KismetSystemLibrary.Delay` 1.5)
  (`/Game/Instructions_Tasks/Connection/BP_Connection_Child.Press Connection Child` (`|GetArrayItem` (`self.Left Children`)) false)
  (`KismetSystemLibrary.Delay` 0.5)
  (for _array_element (`self.Right Children`)
    (if (== (`/Game/Instructions_Tasks/Connection/BP_Connection_Child.Value` (`|GetArrayItem` (`self.Left Children`))) (`/Game/Instructions_Tasks/Connection/BP_Connection_Child.Value` _array_element))
      (`/Game/Instructions_Tasks/Connection/BP_Connection_Child.Press Connection Child` _array_element false)))
  (`KismetSystemLibrary.Delay` 1.0)
  (`/Game/Instructions_Tasks/Connection/BP_Connection_Child.Press Connection Child` (`|GetArrayItem` (`self.Left Children`) 1) false)
  (`KismetSystemLibrary.Delay` 0.5)
  (for _array_element_2 (`self.Right Children`)
    (if (== (`/Game/Instructions_Tasks/Connection/BP_Connection_Child.Value` (`|GetArrayItem` (`self.Left Children`) 1)) (`/Game/Instructions_Tasks/Connection/BP_Connection_Child.Value` _array_element_2))
      (`/Game/Instructions_Tasks/Connection/BP_Connection_Child.Press Connection Child` _array_element_2 false)))
  (`KismetSystemLibrary.Delay` 1.0)
  (`/Game/Instructions_Tasks/Connection/BP_Connection_Child.Press Connection Child` (`|GetArrayItem` (`self.Left Children`) 2) false)
  (`KismetSystemLibrary.Delay` 0.5)
  (for _array_element_3 (`self.Right Children`)
    (if (== (`/Game/Instructions_Tasks/Connection/BP_Connection_Child.Value` (`|GetArrayItem` (`self.Left Children`) 2)) (`/Game/Instructions_Tasks/Connection/BP_Connection_Child.Value` _array_element_3))
      (`/Game/Instructions_Tasks/Connection/BP_Connection_Child.Press Connection Child` _array_element_3 false)))
  (`KismetSystemLibrary.Delay` 1.0)
  (for _array_element_4 (`self.Left Children`)
    (`/Game/Instructions_Tasks/Connection/BP_Connection_Child.Reset Connection Child` _array_element_4))
  (for _array_element_5 (`self.Right Children`)
    (`/Game/Instructions_Tasks/Connection/BP_Connection_Child.Reset Connection Child` _array_element_5))
  (`self.Start Instruction Countdown` _instructiontime)
  (bind _asbp_player (cast `/Game/Player/Blueprints/BP_Player` (`GameplayStatics.GetPlayerCharacter` 0)))
  (`/Game/UI/In-Game/WBP_HUD.Start Timer` (`/Game/Player/Blueprints/BP_Player.HUD` _asbp_player) _instructiontime)
  (set `self.Solution Being Shown` false)
  (set `self.Solution Shown` true))

(fn `Complete Instruction`
  (params (Successful :type Boolean))
  (`parent.Complete Instruction` Successful)
  (for _array_element (`self.Left Children`)
    (`self.SetActorEnableCollision` _array_element false))
  (for _array_element_2 (`self.Right Children`)
    (`self.SetActorEnableCollision` _array_element_2 false)))

(fn `Enable Instruction`
  (bind ((`InstructionType_2_6A9FB7814C2D0346CFAC84934FEBBF4F` _instructiontype) (`InstructionTime_32_0CE54A424D1941F04ADBD48A30216293` _instructiontime)) (break `/Game/Instructions_Tasks/Struct_Instruction_Info` (`self.Instruction Info`)))
  (`parent.Enable Instruction`)
  (`/Game/Instructions_Tasks/Connection/BP_Connection_Child.Reset Connection Child` (`self.Left Children`))
  (`/Game/Instructions_Tasks/Connection/BP_Connection_Child.Reset Connection Child` (`self.Right Children`))
  (for _array_element (`self.Left Children`)
    (`self.SetActorEnableCollision` _array_element true))
  (for _array_element_2 (`self.Right Children`)
    (`self.SetActorEnableCollision` _array_element_2 true))
  (if (`self.Solution Shown`)
    (`self.Start Instruction Countdown` _instructiontime)
    (bind _asbp_player (cast `/Game/Player/Blueprints/BP_Player` (`GameplayStatics.GetPlayerCharacter` 0)))
    (`/Game/UI/In-Game/WBP_HUD.Start Timer` (`/Game/Player/Blueprints/BP_Player.HUD` _asbp_player) _instructiontime)))

(fn `First Time Show`
  (`parent.First Time Show`)
  (`self.Show Connection Solution`))

(fn `Setup Instruction`
  (params (`Instruction Info` :type "/Game/Instructions_Tasks/Struct_Instruction_Info Structure"))
  (locals (`Current Random Left` :type "/Game/Instructions_Tasks/Connection/BP_Connection_Child Object Reference") (`Current Random Right` :type "/Game/Instructions_Tasks/Connection/BP_Connection_Child Object Reference"))
  (`self.Initialise Left and Right Children`)
  (`parent.Setup Instruction` `Instruction Info`))

(fn `UserConstructionScript`
  (`parent.UserConstructionScript`))