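; Typing instruction task Blueprint that has the player type a required text into a UI widget.
; Enabling it creates or reuses WBP_Typing_Instruction, resets it and switches controls to UI input focused on the widget.
; A submitted word matching the instruction's correct text completes the interaction; a mismatch clears the field, each with audio feedback.
; Completion or countdown end removes the widget and restores standard movement controls.
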(event `Word Submitted`
  (params (`Text Submitted` :type Text))
  (if (== `Text Submitted` (`.CorrectText_2_A6DEAB874957CD73429E54A751E2C9E0` (break `/Game/Instructions_Tasks/Typing/Struct_Typing_Instruction_Info` (`.TypingInstructionInfo_26_737AAD5E43CCEF135DB9C98F907009F9` (break `/Game/Instructions_Tasks/Struct_Instruction_Info` (`self.Instruction Info`))))))
    (`self.Instruction Interact` true)
    (`FMODBlueprintStatics.PlayEvent2D` "/Game/FMOD/Events/In-Game/Typing_Entered.Typing_Entered")
    (else
      (`/Game/UI/In-Game/WBP_Typing_Instruction.Reset Text` (`self.Created Widget`))
      (`FMODBlueprintStatics.PlayEvent2D` "/Game/FMOD/Events/In-Game/Typing_Incorrect.Typing_Incorrect"))))

(fn `Complete Instruction`
  (params (Successful :type Boolean))
  (`KismetSystemLibrary.PrintString` "COMPLETED INSTRUCTION TYPING")
  (`Widget.RemoveFromParent` (`self.Created Widget`))
  (message `/Game/Player/Blueprints/BPI_Player_Controller.Update Controls` (`GameplayStatics.GetPlayerController` 0) "/Game/Player/Input/IMC_Standard_Moving.IMC_Standard_Moving" null)
  (`parent.Complete Instruction` Successful))

(fn `Enable Instruction`
  (bind _created_widget (`self.Created Widget`))
  (`parent.Enable Instruction`)
  (`KismetSystemLibrary.PrintString` "ENABLE INSTRUCTION TYPING")
  (`/Engine/EditorBlueprintResources/StandardMacros.IsValid` (`self.Created Widget`)
    (:`Is Valid`
      _)
    (:`Is Not Valid`
      (bind _returnvalue (`|CreateWidget` "/Game/UI/In-Game/WBP_Typing_Instruction.WBP_Typing_Instruction_C" null self))
      (set `self.Created Widget` _returnvalue)))
  (`/Game/UI/In-Game/WBP_Typing_Instruction.Reset Text` _created_widget)
  (`UserWidget.AddToViewport` _created_widget 0)
  (message `/Game/Player/Blueprints/BPI_Player_Controller.Update Controls` (`GameplayStatics.GetPlayerController` 0) "/Game/Player/Input/IMC_UI.IMC_UI" _created_widget))

(fn `Finish Instruction Countdown`
  (`parent.Finish Instruction Countdown`)
  (`KismetSystemLibrary.PrintString` "COMPLETED INSTRUCTION TYPING")
  (`Widget.RemoveFromParent` (`self.Created Widget`))
  (message `/Game/Player/Blueprints/BPI_Player_Controller.Update Controls` (`GameplayStatics.GetPlayerController` 0) "/Game/Player/Input/IMC_Standard_Moving.IMC_Standard_Moving" null))

(fn `Setup Instruction`
  (params (`Instruction Info` :type "/Game/Instructions_Tasks/Struct_Instruction_Info Structure"))
  (`parent.Setup Instruction` `Instruction Info`))

(fn `UserConstructionScript`
  (`parent.UserConstructionScript`))