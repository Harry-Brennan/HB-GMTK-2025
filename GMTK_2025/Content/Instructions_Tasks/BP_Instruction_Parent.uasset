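; Base actor for timed player instruction tasks, configured by an InstructionInfo struct that sets its type and transform.
; Enabling shows it with type-dependent spawn feedback and starts a countdown mirrored on the player HUD, except for Connection and Match.
; Interaction stops the timer, then plays the Button child's animation or completes other types, hiding the actor and broadcasting the result.
; Timeout costs a life and reports failure, except for Colour.
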(fn `Complete Instruction`
  (params (Successful :type Boolean :default true))
  (`self.SetActorEnableCollision` false)
  (`self.SetActorHiddenInGame` true)
  (set `self.Active` false)
  (`self.Stop Instruction Countdown`)
  (`self.Instruction Complete ED` (`self.Instruction Info`) self Successful))

(fn `Disable Instruction`
  (set `self.Active` false))

(fn `Enable Instruction`
  (bind ((`InstructionType_2_6A9FB7814C2D0346CFAC84934FEBBF4F` _instructiontype) (`InstructionTime_32_0CE54A424D1941F04ADBD48A30216293` _instructiontime)) (break `/Game/Instructions_Tasks/Struct_Instruction_Info` (`self.Instruction Info`)))
  (set `self.Active` true)
  (if (not (or (`|EnumEquality` _instructiontype "NewEnumerator2") (`|EnumEquality` _instructiontype "NewEnumerator5")))
    (`FMODBlueprintStatics.PlayEventAtLocation` "/Game/FMOD/Events/In-Game/Instruction_Spawn.Instruction_Spawn" (`KismetMathLibrary.MakeTransform` (`self.K2_GetActorLocation`)))
    (`LegacyCameraShake.StartLegacyCameraShake` (`GameplayStatics.GetPlayerCameraManager` 0) "/Game/Instructions_Tasks/BP_Instruction_Spawned_CS.BP_Instruction_Spawned_CS_C"))
  (`self.SetActorEnableCollision` true)
  (`self.SetActorHiddenInGame` false)
  (if (not (or (`|EnumEquality` _instructiontype "NewEnumerator7") (`|EnumEquality` _instructiontype "NewEnumerator3")))
    (`self.Start Instruction Countdown` _instructiontime)
    (bind _asbp_player (cast `/Game/Player/Blueprints/BP_Player` (`GameplayStatics.GetPlayerCharacter` 0)))
    (`/Game/UI/In-Game/WBP_HUD.Start Timer` (`/Game/Player/Blueprints/BP_Player.HUD` _asbp_player) _instructiontime)))

(fn `Finish Instruction Countdown`
  (`KismetSystemLibrary.PrintString` "Instruction Countdown Over")
  (`self.Instruction Countdown End`)
  (bind _asbp_player (cast `/Game/Player/Blueprints/BP_Player` (`GameplayStatics.GetPlayerCharacter` 0)))
  (`/Game/UI/In-Game/WBP_HUD.Stop Timer` (`/Game/Player/Blueprints/BP_Player.HUD` _asbp_player))
  (if (not (`|EnumEquality` (`.InstructionType_2_6A9FB7814C2D0346CFAC84934FEBBF4F` (break `/Game/Instructions_Tasks/Struct_Instruction_Info` (`self.Instruction Info`))) "NewEnumerator1"))
    (bind _asbp_player_2 (cast `/Game/Player/Blueprints/BP_Player` (`GameplayStatics.GetPlayerCharacter` 0)))
    (`/Game/Player/Blueprints/BP_Player.Decrease Life` _asbp_player_2)
    (`self.Instruction Complete ED` (`self.Instruction Info`) self)
    (`self.SetActorEnableCollision` false)
    (`self.SetActorHiddenInGame` true)
    (set `self.Active` false)))

(fn `First Time Show`)

(fn `Instruction Interact`
  (params (Successful :type Boolean))
  (if (`self.Active`)
    (`self.Stop Instruction Countdown`)
    (switch `/Game/Instructions_Tasks/Enum_Instruction_Types` (`.InstructionType_2_6A9FB7814C2D0346CFAC84934FEBBF4F` (break `/Game/Instructions_Tasks/Struct_Instruction_Info` (`self.Instruction Info`)))
      (:`NewEnumerator0`
        (bind _asbp_button_instruction (cast `/Game/Instructions_Tasks/Buttons/BP_Button_Instruction` self))
        (`/Game/Instructions_Tasks/Buttons/BP_Button_Instruction.Button Interact Anim` _asbp_button_instruction))
      (:`NewEnumerator1`
        (`self.Complete Instruction` Successful :!label _label))
      (:`NewEnumerator2`
        (goto _label))
      (:`NewEnumerator3`
        (goto _label))
      (:`NewEnumerator4`
        (goto _label))
      (:`NewEnumerator5`
        (goto _label))
      (:`NewEnumerator6`
        (goto _label))
      (:`NewEnumerator7`
        (goto _label)))))

(fn `Setup Instruction`
  (params (`Instruction Info` :type "/Game/Instructions_Tasks/Struct_Instruction_Info Structure"))
  (bind _output_get (set `self.Instruction Info` `Instruction Info`))
  (bind ((`InstructionType_2_6A9FB7814C2D0346CFAC84934FEBBF4F` _instructiontype) (`InstructionWorldTranform_9_3009BF554967D21A40A6328E565A667E` _instructionworldtranform)) (break `/Game/Instructions_Tasks/Struct_Instruction_Info` _output_get))
  (`self.K2_SetActorTransform` _instructionworldtranform)
  (if (not (or (`|EnumEquality` _instructiontype "NewEnumerator2") (`|EnumEquality` _instructiontype "NewEnumerator5")))
    (`FMODBlueprintStatics.PlayEventAtLocation` "/Game/FMOD/Events/In-Game/Instruction_Spawn.Instruction_Spawn" (`KismetMathLibrary.MakeTransform` (`self.K2_GetActorLocation`)))))

(fn `Start Instruction Countdown`
  (params (`Total Instruction Time` :type "Float (double-precision)"))
  (bind _returnvalue (`KismetSystemLibrary.K2_SetTimer` null "Finish Instruction Countdown" `Total Instruction Time`))
  (set `self.Instruction Countdown Timer` _returnvalue))

(fn `Stop Instruction Countdown`
  (`KismetSystemLibrary.K2_ClearAndInvalidateTimerHandle` (`self.Instruction Countdown Timer`))
  (bind _asbp_player (cast `/Game/Player/Blueprints/BP_Player` (`GameplayStatics.GetPlayerCharacter` 0)))
  (`/Game/UI/In-Game/WBP_HUD.Stop Timer` (`/Game/Player/Blueprints/BP_Player.HUD` _asbp_player)))

(fn `UserConstructionScript`)