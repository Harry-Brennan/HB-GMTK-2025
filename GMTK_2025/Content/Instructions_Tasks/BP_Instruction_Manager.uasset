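; Instruction manager that runs a level's growing, Simon-style loop of timed player tasks, from start countdown to level-over screen.
; At BeginPlay it randomises task placement from tagged TargetPoints, first pre-generating a long random list for the endless map.
; It spawns each new instruction with a popup, re-enables earlier ones each loop and sends successes to the score manager.
; The tutorial map adds opening and closing dialogue, and progression halts when player lives run out.
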(event `self.ReceiveBeginPlay`
  (`|ExecutionSequence`
    (:`then_0`
      (if (`|EnumEquality` (`self.Map Name`) "NewEnumerator4")
        (bind _output_get (set `self.Max Instruction Count` 400))
        (`KismetArrayLibrary.Array_Clear` (`self.Intended Instructions Data`))
        (for _ (range (+ _output_get 1))
          (set `self.Current Spawning Endless Instruction Type` (`KismetArrayLibrary.Array_Random` (`|MakeArray` "NewEnumerator0" "NewEnumerator1" "NewEnumerator2" "NewEnumerator3" "NewEnumerator4" "NewEnumerator5" "NewEnumerator6" "NewEnumerator7" :!type "/Game/Instructions_Tasks/Enum_Instruction_Types Enum")))
          (`KismetArrayLibrary.Array_Add` (`self.Intended Instructions Data`) (make `/Game/Instructions_Tasks/Struct_Instruction_Info` (`self.Current Spawning Endless Instruction Type`) "0.000000,0.000000,0.000000|0.000000,0.000000,0.000000|1.000000,1.000000,1.000000" (/ (`KismetMathLibrary.Conv_IntToDouble` (`KismetMathLibrary.FFloor` (* (`KismetMathLibrary.SelectFloat` (`KismetMathLibrary.RandomFloatInRange` 1.5 2.5) (`KismetMathLibrary.RandomFloatInRange` 4.0 6.0) (`|EnumEquality` (`self.Current Spawning Endless Instruction Type`) "NewEnumerator1")) 10.0))) 10.0) (struct) (make `/Game/Instructions_Tasks/Matches/Struct_Match_Info` (`KismetMathLibrary.RandomIntegerInRange` 5 9) (`KismetArrayLibrary.Array_Random` (`|MakeArray` "NewEnumerator0" "NewEnumerator1" "NewEnumerator2" :!type "/Game/Instructions_Tasks/Matches/Enum_Match_Types Enum"))) (make `/Game/Instructions_Tasks/Colours/Struct_Colour_Instruction_Info` (`KismetMathLibrary.RandomIntegerInRange` 0 3)) (make `/Game/Instructions_Tasks/Shapes/Struct_Shape_Instruction_Info` (`KismetArrayLibrary.Array_Random` (`|MakeArray` "NewEnumerator0" "NewEnumerator1" "NewEnumerator2" "NewEnumerator3" "NewEnumerator4" :!type "/Game/Instructions_Tasks/Shapes/Enum_Shapes Enum"))) (make `/Game/Instructions_Tasks/Typing/Struct_Typing_Instruction_Info` (`KismetTextLibrary.Conv_StringToText` (`|GetEnumeratorNameAsString` (cast `/Game/Instructions_Tasks/Typing/Enum_Possible_Typing_Words` (`KismetMathLibrary.Conv_IntToByte` (`KismetMathLibrary.RandomIntegerInRange` 0 (- (enumcount `/Game/Instructions_Tasks/Typing/Enum_Possible_Typing_Words`) 1))))))) (make `/Game/Instructions_Tasks/Selection/Struct_Selection_Instruction_Info` (`KismetArrayLibrary.Array_Random` (`|MakeArray` "NewEnumerator0" "NewEnumerator1" "NewEnumerator2" "NewEnumerator3" :!type "/Game/Instructions_Tasks/Selection/Enum_Selection_Instruction_Types Enum")) (`|MakeArray` "NewEnumerator0" "NewEnumerator1" "NewEnumerator2" "NewEnumerator3" :!type "/Game/Instructions_Tasks/Selection/Enum_Selection_Instruction_Types Enum")))))
        (`self.Initialise All Instruction Transforms`)
        (else
          (set `self.Max Instruction Count` (`KismetArrayLibrary.Array_Length` (`self.Intended Instructions Data`)))
          (`self.Initialise All Instruction Transforms`))))
    (:`then_1`
      (if (`|EnumEquality` (`self.Map Name`) "NewEnumerator0")
        (`KismetSystemLibrary.Delay` 1.0)
        (bind _asbp_player (cast `/Game/Player/Blueprints/BP_Player` (`GameplayStatics.GetPlayerCharacter` 0)))
        (bind _returnvalue (`|CreateWidget` "/Game/UI/Tutorial/WBP_Tutorial_Dialogue.WBP_Tutorial_Dialogue_C"))
        (`UserWidget.AddToViewport` _returnvalue 0)
        (`/Game/UI/Tutorial/WBP_Tutorial_Dialogue.Show Tutorial Dialogue` _returnvalue)
        (set `/Game/Player/Blueprints/BP_Player.Tutorial Dialogue` _returnvalue _asbp_player)
        (else
          (`Controller.SetIgnoreMoveInput` (`GameplayStatics.GetPlayerController` 0) true :!label _label)
          (`Controller.SetIgnoreLookInput` (`GameplayStatics.GetPlayerController` 0) true)
          (bind _returnvalue_2 (`|CreateWidget` "/Game/UI/In-Game/WBP_Loop_Start_Countdown.WBP_Loop_Start_Countdown_C"))
          (`UserWidget.AddToViewport` _returnvalue_2 0)
          (set `self.Loop Start Countdown` _returnvalue_2))))))

(event `Start Game`
  (goto _label))

(fn `Enable Next Instruction`
  (`KismetSystemLibrary.PrintString` "ENABLE NEXT INSTRUCTION IN INSTRUCTION MANAGER")
  (bind _asbp_player (cast `/Game/Player/Blueprints/BP_Player` (`GameplayStatics.GetPlayerCharacter` 0)))
  (if (not (== (`/Game/Player/Blueprints/BP_Player.Current Life` _asbp_player) 0))
    (bind _result (`/Engine/EditorBlueprintResources/StandardMacros.IncrementInt` (`self.Current Instruction Loop Count`))
      (:`  `
        (`self.Instruction Count Updated ED` _result)
        (bind _returnvalue (- _result 1))
        (`/Game/Instructions_Tasks/BP_Instruction_Parent.Enable Instruction` (`|GetArrayItem` (`self.Instructions List`) _returnvalue))
        (bind ((`InstructionType_2_6A9FB7814C2D0346CFAC84934FEBBF4F` _instructiontype)) (break `/Game/Instructions_Tasks/Struct_Instruction_Info` (`|GetArrayItem` (`self.Intended Instructions Data`) _returnvalue)))
        (if (not (`|EnumEquality` _instructiontype "NewEnumerator5"))
          (message `/Game/Player/Blueprints/BPI_Player_Controller.Update Controls` (`GameplayStatics.GetPlayerController` 0) (select `/Game/Instructions_Tasks/Enum_Instruction_Types` _instructiontype :`NewEnumerator0` "/Game/Player/Input/IMC_Standard_Moving.IMC_Standard_Moving" :`NewEnumerator1` "/Game/Player/Input/IMC_Standard_Moving.IMC_Standard_Moving" :`NewEnumerator2` "/Game/Player/Input/IMC_Standard_Moving.IMC_Standard_Moving" :`NewEnumerator3` "/Game/Player/Input/IMC_Standard_Moving.IMC_Standard_Moving" :`NewEnumerator4` "/Game/Player/Input/IMC_Standard_Moving.IMC_Standard_Moving" :`NewEnumerator6` "/Game/Player/Input/IMC_Standard_Moving.IMC_Standard_Moving" :`NewEnumerator7` "/Game/Player/Input/IMC_Standard_Moving.IMC_Standard_Moving" :!type "InputMappingContext Object Reference") null))))))

(fn `First Instruction Start Loop`
  (`self.Generate New Next Instruction`))

(fn `Generate New Next Instruction`
  (locals (`Current Random Instruction Type` :type "/Game/Instructions_Tasks/Enum_Instruction_Types Enum"))
  (bind ((`InstructionType_2_6A9FB7814C2D0346CFAC84934FEBBF4F` _instructiontype)) (break `/Game/Instructions_Tasks/Struct_Instruction_Info` (`|GetArrayItem` (`self.Intended Instructions Data`) (`self.Current Instruction Loop Count`))))
  (if (not (`|EnumEquality` _instructiontype "NewEnumerator5"))
    (message `/Game/Player/Blueprints/BPI_Player_Controller.Update Controls` (`GameplayStatics.GetPlayerController` 0) (select `/Game/Instructions_Tasks/Enum_Instruction_Types` _instructiontype :`NewEnumerator0` "/Game/Player/Input/IMC_Standard_Moving.IMC_Standard_Moving" :`NewEnumerator1` "/Game/Player/Input/IMC_Standard_Moving.IMC_Standard_Moving" :`NewEnumerator2` "/Game/Player/Input/IMC_Standard_Moving.IMC_Standard_Moving" :`NewEnumerator3` "/Game/Player/Input/IMC_Standard_Moving.IMC_Standard_Moving" :`NewEnumerator4` "/Game/Player/Input/IMC_Standard_Moving.IMC_Standard_Moving" :`NewEnumerator6` "/Game/Player/Input/IMC_Standard_Moving.IMC_Standard_Moving" :`NewEnumerator7` "/Game/Player/Input/IMC_Standard_Moving.IMC_Standard_Moving" :!type "InputMappingContext Object Reference") null))
  (bind _asbp_player (cast `/Game/Player/Blueprints/BP_Player` (`GameplayStatics.GetPlayerCharacter` 0)))
  (if (not (<= (`/Game/Player/Blueprints/BP_Player.Current Life` _asbp_player) 0))
    (switch `/Game/Instructions_Tasks/Enum_Instruction_Types` (`.InstructionType_2_6A9FB7814C2D0346CFAC84934FEBBF4F` (break `/Game/Instructions_Tasks/Struct_Instruction_Info` (`|GetArrayItem` (`self.Intended Instructions Data`) (`self.Current Instruction Loop Count`))))
      (:`NewEnumerator0`
        (bind _returnvalue (`|SpawnActorFromClass` "/Game/Instructions_Tasks/Buttons/BP_Button_Instruction.BP_Button_Instruction_C" (`KismetMathLibrary.MakeTransform` (0.0 0.0 0.0)) "Undefined" "MultiplyWithRoot" null null))
        (`self.Setup Spawned Instruction` _returnvalue))
      (:`NewEnumerator1`
        (bind _returnvalue_2 (`|SpawnActorFromClass` "/Game/Instructions_Tasks/Colours/BP_Colour_Instruction.BP_Colour_Instruction_C" (`KismetMathLibrary.MakeTransform` (0.0 0.0 0.0)) "Undefined" "MultiplyWithRoot" null null))
        (`self.Setup Spawned Instruction` _returnvalue_2))
      (:`NewEnumerator2`
        (bind _returnvalue_3 (`|SpawnActorFromClass` "/Game/Instructions_Tasks/Jumping/BP_Jump_Instruction.BP_Jump_Instruction_C" (`KismetMathLibrary.MakeTransform` (0.0 0.0 0.0)) "Undefined" "MultiplyWithRoot" null null))
        (`self.Setup Spawned Instruction` _returnvalue_3))
      (:`NewEnumerator3`
        (bind _returnvalue_4 (`|SpawnActorFromClass` "/Game/Instructions_Tasks/Matches/BP_Match_Instruction.BP_Match_Instruction_C" (`KismetMathLibrary.MakeTransform` (0.0 0.0 0.0)) "Undefined" "MultiplyWithRoot" null null))
        (`self.Setup Spawned Instruction` _returnvalue_4))
      (:`NewEnumerator4`
        (bind _returnvalue_5 (`|SpawnActorFromClass` "/Game/Instructions_Tasks/Shapes/BP_Shape_Instruction.BP_Shape_Instruction_C" (`KismetMathLibrary.MakeTransform` (0.0 0.0 0.0)) "Undefined" "MultiplyWithRoot" null null))
        (`self.Setup Spawned Instruction` _returnvalue_5))
      (:`NewEnumerator5`
        (bind _returnvalue_6 (`|SpawnActorFromClass` "/Game/Instructions_Tasks/Typing/BP_Typing_Instruction.BP_Typing_Instruction_C" (`KismetMathLibrary.MakeTransform` (0.0 0.0 0.0)) "Undefined" "MultiplyWithRoot" null null))
        (`self.Setup Spawned Instruction` _returnvalue_6))
      (:`NewEnumerator6`
        (bind _returnvalue_7 (`|SpawnActorFromClass` "/Game/Instructions_Tasks/Selection/BP_Selection_Instruction.BP_Selection_Instruction_C" (`KismetMathLibrary.MakeTransform` (0.0 0.0 0.0)) "Undefined" "MultiplyWithRoot" null null))
        (`self.Setup Spawned Instruction` _returnvalue_7))
      (:`NewEnumerator7`
        (bind _returnvalue_8 (`|SpawnActorFromClass` "/Game/Instructions_Tasks/Connection/BP_Connection_Instruction.BP_Connection_Instruction_C" (`KismetMathLibrary.MakeTransform` (0.0 0.0 0.0)) "Undefined" "MultiplyWithRoot" null null))
        (`self.Setup Spawned Instruction` _returnvalue_8)))))

(fn `Initialise All Instruction Transforms`
  (locals (`All Target Points` :type "Array of TargetPoint Object Reference") (`Button Transform` :type "Array of Transform Structure") (`Selection Transform` :type "Array of Transform Structure") (`Connection Transform` :type "Array of Transform Structure") (`Shape Transform` :type "Array of Transform Structure") (`Colour Transform` :type "Array of Transform Structure") (`Matches Transform` :type "Array of Transform Structure") (`Shapes Transform` :type "Array of Transform Structure"))
  (bind _returnvalue (`KismetMathLibrary.MakeTransform` (0.0 0.0 0.0)))
  (bind _outactors (`GameplayStatics.GetAllActorsOfClass` "/Script/Engine.TargetPoint"))
  (bind _output_get (set `local.All Target Points` _outactors))
  (for _array_element _output_get
    (switch `name` (`|GetArrayItem` (`Actor.Tags` _array_element))
      (:`Button`
        (bind _returnvalue_2 (`self.GetTransform` _array_element))
        (`KismetArrayLibrary.Array_Add` (`local.Button Transform`) _returnvalue_2))
      (:`Selection`
        (`KismetArrayLibrary.Array_Add` (`local.Selection Transform`) _returnvalue_2))
      (:`Connection`
        (`KismetArrayLibrary.Array_Add` (`local.Connection Transform`) _returnvalue_2))
      (:`Shapes`
        (`KismetArrayLibrary.Array_Add` (`local.Shape Transform`) _returnvalue_2))
      (:`Colour`
        (`KismetArrayLibrary.Array_Add` (`local.Colour Transform`) _returnvalue_2))
      (:`Matches`
        (`KismetArrayLibrary.Array_Add` (`local.Matches Transform`) _returnvalue_2))))
  (for (_array_element_2 _array_index) (`self.Intended Instructions Data`)
    (bind _structout (setmembers `/Game/Instructions_Tasks/Struct_Instruction_Info` :`StructRef` _array_element_2 :`Instruction World Tranform` (select `/Game/Instructions_Tasks/Enum_Instruction_Types` (`.InstructionType_2_6A9FB7814C2D0346CFAC84934FEBBF4F` (break `/Game/Instructions_Tasks/Struct_Instruction_Info` _array_element_2)) :`NewEnumerator0` (`KismetArrayLibrary.Array_Random` (`local.Button Transform`)) :`NewEnumerator1` (`KismetArrayLibrary.Array_Random` (`local.Colour Transform`)) :`NewEnumerator2` _returnvalue :`NewEnumerator3` (`KismetArrayLibrary.Array_Random` (`local.Matches Transform`)) :`NewEnumerator4` (`KismetArrayLibrary.Array_Random` (`local.Shape Transform`)) :`NewEnumerator5` _returnvalue :`NewEnumerator6` (`KismetArrayLibrary.Array_Random` (`local.Selection Transform`)) :`NewEnumerator7` (`KismetArrayLibrary.Array_Random` (`local.Connection Transform`))) :`Typing Instruction Info` (make `/Game/Instructions_Tasks/Typing/Struct_Typing_Instruction_Info` (`KismetTextLibrary.Conv_StringToText` (`|GetEnumeratorNameAsString` (cast `/Game/Instructions_Tasks/Typing/Enum_Possible_Typing_Words` (`KismetMathLibrary.Conv_IntToByte` (`KismetMathLibrary.RandomIntegerInRange` 0 (- (enumcount `/Game/Instructions_Tasks/Typing/Enum_Possible_Typing_Words`) 1)))))))))
    (`KismetArrayLibrary.Array_Set` (`self.Intended Instructions Data`) _array_index _structout)))

(fn `Instruction Completed`
  (params (`Instruction Info` :type "/Game/Instructions_Tasks/Struct_Instruction_Info Structure") (`Instruction Ref` :type "/Game/Instructions_Tasks/BP_Instruction_Parent Object Reference") (Successful :type Boolean))
  (bind _instructions_list (`self.Instructions List`))
  (bind ((`InstructionType_2_6A9FB7814C2D0346CFAC84934FEBBF4F` _instructiontype) (`InstructionTime_32_0CE54A424D1941F04ADBD48A30216293` _instructiontime)) (break `/Game/Instructions_Tasks/Struct_Instruction_Info` (`local.Instruction Info`)))
  (bind _asbp_player (cast `/Game/Player/Blueprints/BP_Player` (`GameplayStatics.GetPlayerCharacter` 0)))
  (if (not (<= (`/Game/Player/Blueprints/BP_Player.Current Life` _asbp_player) 0))
    (`KismetSystemLibrary.PrintString` "INSTRUCTION COMPLETE")
    (if (`local.Successful`)
      (`FMODBlueprintStatics.PlayEvent2D` "/Game/FMOD/Events/In-Game/Instruction_Passed.Instruction_Passed")
      (bind _asbp_player_2 (cast `/Game/Player/Blueprints/BP_Player` (`GameplayStatics.GetPlayerCharacter` 0)))
      (`/Game/Instructions_Tasks/BP_Score_Manager.Score Calculation` (`self.Score Manager Ref`) _instructiontype (`self.Current Instruction Loop Count`) (`/Game/UI/In-Game/WBP_Instruction_Timer.Current Timer Value` (`/Game/UI/In-Game/WBP_HUD.WBP_Instruction_Timer` (`/Game/Player/Blueprints/BP_Player.HUD` _asbp_player_2))) _instructiontime))
    (`/Engine/EditorBlueprintResources/StandardMacros.IsValid` (`self.Newly Created Instruction`)
      (:`Is Valid`
        (if (== (`self.Current Instructions Count`) (`self.Max Instruction Count`))
          (if (`|EnumEquality` (`self.Map Name`) "NewEnumerator0")
            (bind _returnvalue (`|CreateWidget` "/Game/UI/Tutorial/WBP_Tutorial_Dialogue.WBP_Tutorial_Dialogue_C" null true))
            (`UserWidget.AddToViewport` _returnvalue 0)
            (message `/Game/Player/Blueprints/BPI_Player_Controller.Update Controls` (`GameplayStatics.GetPlayerController` 0) "/Game/Player/Input/IMC_Tutorial.IMC_Tutorial" _returnvalue)
            (`/Game/UI/Tutorial/WBP_Tutorial_Dialogue.Show Tutorial Dialogue` _returnvalue)
            (bind _asbp_player_3 (cast `/Game/Player/Blueprints/BP_Player` (`GameplayStatics.GetPlayerCharacter` 0)))
            (set `/Game/Player/Blueprints/BP_Player.Tutorial Dialogue` _returnvalue _asbp_player_3)
            (else
              (bind _returnvalue_2 (`|CreateWidget` "/Game/UI/Menus/WBP_Level_Over.WBP_Level_Over_C" null true))
              (`UserWidget.AddToViewport` _returnvalue_2 0)
              (message `/Game/Player/Blueprints/BPI_Player_Controller.Update Controls` (`GameplayStatics.GetPlayerController` 0) "/Game/Player/Input/IMC_UI.IMC_UI" _returnvalue_2)))
          (else
            (bind _returnvalue_3 (`|CreateWidget` "/Game/UI/In-Game/WBP_Loop_Popup.WBP_Loop_Popup_C"))
            (`UserWidget.AddToViewport` _returnvalue_3 0))))
      (:`Is Not Valid`
        (if (== (`KismetArrayLibrary.Array_LastIndex` _instructions_list) (`KismetArrayLibrary.Array_Find` _instructions_list (`local.Instruction Ref`)))
          (`KismetSystemLibrary.K2_SetTimer` null "Generate New Next Instruction" 1.0)
          (else
            (`KismetSystemLibrary.K2_SetTimer` null "Enable Next Instruction" 1.0)))))))

(fn `Popup Animation FInished`
  (params (`Instruction Ref` :type "/Game/Instructions_Tasks/BP_Instruction_Parent Object Reference"))
  (`/Game/Instructions_Tasks/BP_Instruction_Parent.Enable Instruction` `Instruction Ref`))

(fn `Restart Loop`
  (bind _asbp_player (cast `/Game/Player/Blueprints/BP_Player` (`GameplayStatics.GetPlayerCharacter` 0)))
  (if (not (<= (`/Game/Player/Blueprints/BP_Player.Current Life` _asbp_player) 0))
    (set `self.Current Instruction Loop Count` 0)
    (`self.Instruction Count Updated ED` 1)
    (set `self.Newly Created Instruction` null)
    (`self.Enable Next Instruction`)))

(fn `Setup Spawned Instruction`
  (params (`Instruction REF` :type "/Game/Instructions_Tasks/BP_Instruction_Parent Object Reference"))
  (`self.SetActorHiddenInGame` `Instruction REF` true)
  (`KismetArrayLibrary.Array_Add` (`self.Instructions List`) `Instruction REF`)
  (`/Engine/EditorBlueprintResources/StandardMacros.IncrementInt` (`self.Current Instructions Count`)
    (:`  `
      (add `/Game/Instructions_Tasks/BP_Instruction_Parent.Instruction Complete ED` (`local.Instruction REF`) (`|CreateDelegate` :!event `Instruction Completed`))
      (`/Game/Instructions_Tasks/BP_Instruction_Parent.Setup Instruction` (`local.Instruction REF`) (`|GetArrayItem` (`self.Intended Instructions Data`) (`self.Current Instruction Loop Count`)))
      (bind _output_get (set `self.Newly Created Instruction` (`local.Instruction REF`)))
      (bind _returnvalue (`|CreateWidget` "/Game/UI/In-Game/WBP_Instruction_Type_Popup.WBP_Instruction_Type_Popup_C"))
      (`UserWidget.AddToViewport` _returnvalue 0)
      (`/Game/UI/In-Game/WBP_Instruction_Type_Popup.Show Popup` _returnvalue (`|GetArrayItem` (`self.Intended Instructions Data`) (`self.Current Instruction Loop Count`)) _output_get)
      (bind _result (`/Engine/EditorBlueprintResources/StandardMacros.IncrementInt` (`self.Current Instruction Loop Count`))
        (:`  `
          (`self.Instruction Count Updated ED` _result)
          (`/Game/Instructions_Tasks/BP_Instruction_Parent.First Time Show` (`local.Instruction REF`)))))))

(fn `UserConstructionScript`)