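; Pressable button instruction that completes its task once the press animation finishes.
; Interaction, guarded against overlapping presses, plays a sound and camera shake while a timeline moves the upper mesh along Z, then calls CompleteInstruction on finish.
; Setup extends the parent instruction logic by resetting the mesh to its raised position.
; Outline highlighting toggles an overlay material on the upper mesh.
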(event `Button Interact Anim`
  (if (not (`self.Button Pressing`))
    (set `self.Button Pressing` true)
    (`FMODBlueprintStatics.PlayEventAtLocation` "/Game/FMOD/Events/In-Game/Object_Pressed.Object_Pressed" (`KismetMathLibrary.MakeTransform` (`self.K2_GetActorLocation`)))
    (`LegacyCameraShake.StartLegacyCameraShake` (`GameplayStatics.GetPlayerCameraManager` 0) "/Game/Instructions_Tasks/BP_Object_Pressed_CS.BP_Object_Pressed_CS_C" 2.0)
    (bind (_direction _alpha) (`Timeline|Button Press Timeline` :!via `PlayFromStart`)
      (:`Update`
        (`SceneComponent.K2_SetRelativeLocation` (`self.Button Upper Mesh`) (`KismetMathLibrary.VLerp` (0.0 0.0 10.0) (0.0 0.0 2.0) _alpha) false false))
      (:`Finished`
        (`self.Complete Instruction` true)
        (set `self.Button Pressing` false)))))

(event `/Game/Instructions_Tasks/BPI_Outlineable.Deactivate_Outline`
  (`MeshComponent.SetOverlayMaterial` (`self.Button Upper Mesh`) null))

(event `/Game/Instructions_Tasks/BPI_Outlineable.Activate_Outline`
  (`MeshComponent.SetOverlayMaterial` (`self.Button Upper Mesh`) "/Game/Assets/M_Outline.M_Outline"))

(fn `Setup Instruction`
  (params (`Instruction Info` :type "/Game/Instructions_Tasks/Struct_Instruction_Info Structure"))
  (`parent.Setup Instruction` `Instruction Info`)
  (`SceneComponent.K2_SetRelativeLocation` (`self.Button Upper Mesh`) (0.0 0.0 10.0) false false))

(fn `UserConstructionScript`
  (`parent.UserConstructionScript`))