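; BP_Score_Manager keeps the player's score for instruction tasks.
; ScoreCalculation picks a base value by instruction type, scales it by the fraction of time remaining, floors it and multiplies by the chain count.
; Colour instructions are the exception, earning a flat base times chain count with no time scaling.
; UpdateScore stores the new total and broadcasts it through the ScoreUpdated event dispatcher.
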(event `Score Calculation`
  (params (`Instruction Type` :type "/Game/Instructions_Tasks/Enum_Instruction_Types Enum" :default "NewEnumerator0") (`Instruction Chain Count` :type Integer) (`Instruction Time Remaining` :type "Float (double-precision)") (`Instruction Total Time` :type "Float (double-precision)"))
  (bind _returnvalue (/ `Instruction Time Remaining` `Instruction Total Time`))
  (`self.Update Score` (+ (`self.Current Player Score`) (select `/Game/Instructions_Tasks/Enum_Instruction_Types` `Instruction Type` :`NewEnumerator0` (* (`KismetMathLibrary.FFloor` (* 25.0 _returnvalue)) `Instruction Chain Count`) :`NewEnumerator1` (* 50 `Instruction Chain Count`) :`NewEnumerator2` (* (`KismetMathLibrary.FFloor` (* 50.0 _returnvalue)) `Instruction Chain Count`) :`NewEnumerator3` (* (`KismetMathLibrary.FFloor` (* 150.0 _returnvalue)) `Instruction Chain Count`) :`NewEnumerator4` (* (`KismetMathLibrary.FFloor` (* 75.0 _returnvalue)) `Instruction Chain Count`) :`NewEnumerator5` (* (`KismetMathLibrary.FFloor` (* 75.0 _returnvalue)) `Instruction Chain Count`) :`NewEnumerator6` (* (`KismetMathLibrary.FFloor` (* 125.0 _returnvalue)) `Instruction Chain Count`) :`NewEnumerator7` (* (`KismetMathLibrary.FFloor` (* 150.0 _returnvalue)) `Instruction Chain Count`)))))

(event `Update Score`
  (params (`New Score` :type Integer))
  (bind _output_get (set `self.Current Player Score` `New Score`))
  (`self.Score Updated ED` _output_get))

(fn `UserConstructionScript`)