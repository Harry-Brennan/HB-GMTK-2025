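; BP_Selection_Arrow is a pressable arrow that steps through options in a selection instruction.
; Pressing it plays a sound and camera shake, then casts its parent actor to BP_Selection_Instruction and calls the next or previous selection handler based on its Next flag.
; Separate events apply or clear an outline overlay material on the arrow mesh to highlight it.
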(event `Press Arrow`
  (`FMODBlueprintStatics.PlayEventAtLocation` "/Game/FMOD/Events/In-Game/Object_Pressed.Object_Pressed" (`KismetMathLibrary.MakeTransform` (`self.K2_GetActorLocation`)))
  (`LegacyCameraShake.StartLegacyCameraShake` (`GameplayStatics.GetPlayerCameraManager` 0) "/Game/Instructions_Tasks/BP_Object_Pressed_CS.BP_Object_Pressed_CS_C")
  (bind _asbp_selection_instruction (cast `/Game/Instructions_Tasks/Selection/BP_Selection_Instruction` (`self.GetParentActor`)))
  (if (`self.Next?`)
    (`/Game/Instructions_Tasks/Selection/BP_Selection_Instruction.Next Selection Button Pressed` _asbp_selection_instruction)
    (else
      (`/Game/Instructions_Tasks/Selection/BP_Selection_Instruction.Previous Selection Button Pressed` _asbp_selection_instruction))))

(event `Deactivate_Outline_1`
  (`MeshComponent.SetOverlayMaterial` (`self.Arrow SM`) null))

(event `Activate_Outline_1`
  (`MeshComponent.SetOverlayMaterial` (`self.Arrow SM`) "/Game/Assets/M_Outline.M_Outline"))

(fn `UserConstructionScript`)