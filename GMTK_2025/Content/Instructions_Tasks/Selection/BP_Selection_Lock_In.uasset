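; BP_Selection_Lock_In is the confirm button used as a child actor of BP_Selection_Instruction.
; A press only registers while that parent is active and no press is running, then plays a sound event and camera shake.
; A timeline animates the Upper component's height, then tells the parent to choose the current selection and re-enables pressing.
; Separate events toggle an outline overlay material on Upper.
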(event `Lock In Button Press`
  (if (not (`self.Button Pressing?`))
    (bind _asbp_selection_instruction (cast `/Game/Instructions_Tasks/Selection/BP_Selection_Instruction` (`self.GetParentActor`)))
    (if (`/Game/Instructions_Tasks/BP_Instruction_Parent.Active` _asbp_selection_instruction)
      (set `self.Button Pressing?` true)
      (`FMODBlueprintStatics.PlayEventAtLocation` "/Game/FMOD/Events/In-Game/Object_Pressed.Object_Pressed" (`KismetMathLibrary.MakeTransform` (`self.K2_GetActorLocation`)))
      (`LegacyCameraShake.StartLegacyCameraShake` (`GameplayStatics.GetPlayerCameraManager` 0) "/Game/Instructions_Tasks/BP_Object_Pressed_CS.BP_Object_Pressed_CS_C" 1.5)
      (bind (_direction _alpha) (`Timeline|Lock In Button Timeline` :!via `PlayFromStart`)
        (:`Update`
          (`SceneComponent.K2_SetRelativeLocation` (`self.Upper`) (`KismetMathLibrary.VLerp` (0.0 0.0 10.0) (0.0 0.0 0.0) _alpha) false false))
        (:`Finished`
          (bind _asbp_selection_instruction_2 (cast `/Game/Instructions_Tasks/Selection/BP_Selection_Instruction` (`self.GetParentActor`)))
          (`/Game/Instructions_Tasks/Selection/BP_Selection_Instruction.Choose Current Selection` _asbp_selection_instruction_2)
          (set `self.Button Pressing?` false))))))

(event `/Game/Instructions_Tasks/BPI_Outlineable.Deactivate_Outline`
  (`MeshComponent.SetOverlayMaterial` (`self.Upper`) null))

(event `/Game/Instructions_Tasks/BPI_Outlineable.Activate_Outline`
  (`MeshComponent.SetOverlayMaterial` (`self.Upper`) "/Game/Assets/M_Outline.M_Outline"))

(fn `UserConstructionScript`)