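; Selection task instruction where the player cycles icons with next/previous arrows and locks in a choice; wrong answers cost a life.
; Child-actor buttons get collision only from enable until completion.
; Arrow presses move the icon widget, play a sound and timeline nudge, then block input until AllowSelectionChange.
; The widget holds a back-reference to this actor, which steps the selection with wrap-around and checks it against InstructionInfo.
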(event `self.ReceiveBeginPlay`
  (bind _aswbp_selection_icons (cast `/Game/UI/In-Game/WBP_Selection_Icons` (`WidgetComponent.GetWidget` (`self.Current Selection Icon`))))
  (bind _output_get (set `self.As WBP Selection Icons` _aswbp_selection_icons))
  (set `/Game/UI/In-Game/WBP_Selection_Icons.Selection Instruction Parent Ref` self _output_get))

(event `Next Selection Button Pressed`
  (bind _returnvalue (select `bool` (`self.Next Button Pressed?`) :`false` (`self.Previous Arrow Actor`) :`true` (`self.Next Arrow Actor`) :!type "SceneComponent Object Reference"))
  (bind (_relativelocation_x _relativelocation_y _relativelocation_z) (`KismetMathLibrary.BreakVector` (`SceneComponent.RelativeLocation` _returnvalue)))
  (if (`TimelineComponent.IsPlaying` (`self.Button Pressed Timeline`))
    _
    (elif (not (`self.Moving Current Selection`))
      (set `self.Next Button Pressed?` true)
      (`/Game/UI/In-Game/WBP_Selection_Icons.Move Icon Down` (`self.As WBP Selection Icons`))
      (`FMODBlueprintStatics.PlayEventAtLocation` "/Game/FMOD/Events/In-Game/Selection_Changed.Selection_Changed" (`KismetMathLibrary.MakeTransform` (`SceneComponent.K2_GetComponentLocation` (`self.Current Selection Icon`))) :!label _label)
      (bind (_direction _alpha) (`Timeline|Button Pressed Timeline` :!via `PlayFromStart`)
        (:`Update`
          (`SceneComponent.K2_SetRelativeLocation` _returnvalue (`KismetMathLibrary.MakeVector` (`KismetMathLibrary.Lerp` 20.0 10.0 _alpha) _relativelocation_y _relativelocation_z) false false))
        (:`Finished`
          (`self.Move Current Selection`))))))

(event `Previous Selection Button Pressed`
  (if (`TimelineComponent.IsPlaying` (`self.Button Pressed Timeline`))
    _
    (elif (not (`self.Moving Current Selection`))
      (set `self.Next Button Pressed?` false)
      (`/Game/UI/In-Game/WBP_Selection_Icons.Move Icon Up` (`self.As WBP Selection Icons`))
      (goto _label))))

(event `Move Current Selection`
  (set `self.Moving Current Selection` true))

(event `Allow Selection Change`
  (set `self.Next Button Pressed?` false)
  (set `self.Moving Current Selection` false))

(event `Update Current Selection Data`
  (bind (_correctselectiontype _availableselectiontypes) (break `/Game/Instructions_Tasks/Selection/Struct_Selection_Instruction_Info` (`.SelectionInstructionInfo_29_1EE52D1241E1B003F0D1B2BEB845BFF8` (break `/Game/Instructions_Tasks/Struct_Instruction_Info` (`self.Instruction Info`)))))
  (bind _returnvalue (`KismetArrayLibrary.Array_LastIndex` _availableselectiontypes))
  (bind _returnvalue_2 (+ (`KismetArrayLibrary.Array_Find` _availableselectiontypes (`self.Current Selection Data`)) 1))
  (bind _returnvalue_3 (- (`KismetArrayLibrary.Array_Find` _availableselectiontypes (`self.Current Selection Data`)) 1))
  (set `self.Current Selection Data` (`|GetArrayItem` _availableselectiontypes (`KismetMathLibrary.SelectInt` (`KismetMathLibrary.SelectInt` 0 _returnvalue_2 (> _returnvalue_2 _returnvalue)) (`KismetMathLibrary.SelectInt` _returnvalue _returnvalue_3 (< _returnvalue_3 0)) (`self.Next Button Pressed?`)))))

(event `Choose Current Selection`
  (if (`|EnumEquality` (`self.Current Selection Data`) (`.CorrectSelectionType_2_3BFFCE8B4DDC3BFF6AA4018099252538` (break `/Game/Instructions_Tasks/Selection/Struct_Selection_Instruction_Info` (`.SelectionInstructionInfo_29_1EE52D1241E1B003F0D1B2BEB845BFF8` (break `/Game/Instructions_Tasks/Struct_Instruction_Info` (`self.Instruction Info`))))))
    (`self.Instruction Interact` true)
    (else
      (`FMODBlueprintStatics.PlayEventAtLocation` "/Game/FMOD/Events/In-Game/Match_Incorrect.Match_Incorrect" (`KismetMathLibrary.MakeTransform` (`self.K2_GetActorLocation`)))
      (bind _asbp_player (cast `/Game/Player/Blueprints/BP_Player` (`GameplayStatics.GetPlayerCharacter` 0)))
      (`/Game/Player/Blueprints/BP_Player.Decrease Life` _asbp_player)
      (`self.Instruction Interact` false))))

(fn `Complete Instruction`
  (params (Successful :type Boolean))
  (`parent.Complete Instruction` Successful)
  (`self.SetActorEnableCollision` (`ChildActorComponent.ChildActor` (`self.Next Arrow Actor`)) false)
  (`self.SetActorEnableCollision` (`ChildActorComponent.ChildActor` (`self.Previous Arrow Actor`)) false)
  (`self.SetActorEnableCollision` (`ChildActorComponent.ChildActor` (`self.Lock In Actor`)) false))

(fn `Enable Instruction`
  (`parent.Enable Instruction`)
  (set `self.Moving Current Selection` false)
  (`self.SetActorEnableCollision` (`ChildActorComponent.ChildActor` (`self.Next Arrow Actor`)) true)
  (`self.SetActorEnableCollision` (`ChildActorComponent.ChildActor` (`self.Previous Arrow Actor`)) true)
  (`self.SetActorEnableCollision` (`ChildActorComponent.ChildActor` (`self.Lock In Actor`)) true)
  (set `self.Current Selection Data` "NewEnumerator0")
  (`/Game/UI/In-Game/WBP_Selection_Icons.Update Selection Icon to Current Selection Data` (`self.As WBP Selection Icons`)))

(fn `UserConstructionScript`
  (`parent.UserConstructionScript`))