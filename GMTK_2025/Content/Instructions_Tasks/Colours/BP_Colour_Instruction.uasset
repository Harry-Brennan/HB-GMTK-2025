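; Colour-matching instruction that tests which colour the player is standing on when its countdown finishes.
; A downward box trace from the player looks for a BP_Colour_Child and activates it; CheckColourCorrectness compares a supplied child colour with the correct value.
; A match reports success to the parent instruction logic.
; A mismatch or missed trace plays an incorrect sound, removes a life and reports failure.
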(event `Player Colour Standing Check`
  (bind _returnvalue (`self.K2_GetActorLocation` (`GameplayStatics.GetPlayerCharacter` 0)))
  (`KismetSystemLibrary.PrintString` "PLAYER COLOUR STANDING CHECK" true true (struct :`G` 0.66 :`B` 1.0 :`A` 1.0) 999.0)
  (bind (_outhit _returnvalue_2) (`KismetSystemLibrary.BoxTraceSingleForObjects` :`Start` _returnvalue :`End` (- _returnvalue (0.0 0.0 150.0)) :`HalfSize` (32.0 32.0 32.0) :`ObjectTypes` (`|MakeArray` "ObjectTypeQuery8" :!type "EObjectTypeQuery Enum") :`DrawDebugType` "ForDuration"))
  (if _returnvalue_2
    (bind _asbp_colour_child (cast `/Game/Instructions_Tasks/Colours/BP_Colour_Child` (`.HitActor` (`GameplayStatics.BreakHitResult` _outhit))))
    (`/Game/Instructions_Tasks/Colours/BP_Colour_Child.Colour Child Activate` _asbp_colour_child)
    (else
      (`FMODBlueprintStatics.PlayEventAtLocation` "/Game/FMOD/Events/In-Game/Match_Incorrect.Match_Incorrect" (`KismetMathLibrary.MakeTransform` (`self.K2_GetActorLocation` (`GameplayStatics.GetPlayerCharacter` 0))) :!label _label)
      (bind _asbp_player (cast `/Game/Player/Blueprints/BP_Player` (`GameplayStatics.GetPlayerCharacter` 0)))
      (`/Game/Player/Blueprints/BP_Player.Decrease Life` _asbp_player)
      (`self.Instruction Interact` false))))

(event `Check Colour Correctness`
  (params (`Child's Colour` :type Integer))
  (if (== `Child's Colour` (`.CorrectColourValue_2_5A0BAA0F4E44517B78BBAF9A2FBB415C` (break `/Game/Instructions_Tasks/Colours/Struct_Colour_Instruction_Info` (`.ColourInstructionInfo_24_9CE1EA624C47A14C3E1775AF69A37D1D` (break `/Game/Instructions_Tasks/Struct_Instruction_Info` (`self.Instruction Info`))))))
    (`self.Instruction Interact` true)
    (else
      (goto _label))))

(fn `Enable Instruction`
  (`parent.Enable Instruction`))

(fn `Finish Instruction Countdown`
  (`parent.Finish Instruction Countdown`)
  (`self.Player Colour Standing Check`))

(fn `Instruction Interact`
  (params (Successful :type Boolean))
  (`KismetSystemLibrary.PrintString` (`KismetStringLibrary.Conv_BoolToString` Successful))
  (`parent.Instruction Interact` Successful))

(fn `UserConstructionScript`
  (`parent.UserConstructionScript`))