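; BP_Colour_Child is one selectable colour piece in a colour task, reporting its colour to an owning parent when activated.
; The construction script sets the mesh material from ColourValue, choosing among blue, green, red and base materials.
; On ColourChildActivate it prints its name to screen, then passes ColourValue to OwningColourParent's CheckColourCorrectness, leaving validation to the parent.
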(event `Colour Child Activate`
  (`KismetSystemLibrary.PrintString` (`KismetSystemLibrary.GetDisplayName` self) true true (struct :`G` 0.66 :`B` 1.0 :`A` 1.0) 99.0)
  (`/Game/Instructions_Tasks/Colours/BP_Colour_Instruction.Check Colour Correctness` (`self.Owning Colour Parent`) (`self.Colour Value`)))

(fn `UserConstructionScript`
  (`PrimitiveComponent.SetMaterial` (`self.Colour Child SM`) 0 (select `int` (`self.Colour Value`) :`0` "/AnimationSharing/AnimSharingBlue.AnimSharingBlue" :`1` "/AnimationSharing/AnimSharingGreen.AnimSharingGreen" :`2` "/AnimationSharing/AnimSharingRed.AnimSharingRed" :`3` "/AnimationSharing/AnimSharingBase.AnimSharingBase" :!type "MaterialInterface Object Reference")))