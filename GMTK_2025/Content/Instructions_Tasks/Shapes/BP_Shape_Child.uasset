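; BP_Shape_Child is a pressable shape piece, spawned as a child actor of BP_Shape_Instruction, whose mesh is chosen from five shapes by ShapeValue.
; A press plays a sound event and camera shake, then a timeline moves the mesh along Z, ignoring presses while it plays.
; When the timeline finishes, the shape reports itself to the parent instruction actor.
; Outline events toggle an overlay material for highlighting.
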(event `self.ReceiveBeginPlay`
  (bind _asbp_shape_instruction (cast `/Game/Instructions_Tasks/Shapes/BP_Shape_Instruction` (`self.GetParentActor`)))
  (set `self.As BP Shape Instruction` _asbp_shape_instruction)
  (`StaticMeshComponent.SetStaticMesh` (`self.Shape SM`) (select `/Game/Instructions_Tasks/Shapes/Enum_Shapes` (`self.Shape Value`) :`NewEnumerator0` "/Game/Assets/Interactions/SM_Diamond.SM_Diamond" :`NewEnumerator1` "/Game/Assets/Interactions/SM_Triangle.SM_Triangle" :`NewEnumerator2` "/Game/Assets/Interactions/SM_Circle.SM_Circle" :`NewEnumerator3` "/Game/Assets/Interactions/SM_Pentagon.SM_Pentagon" :`NewEnumerator4` "/Game/Assets/Interactions/SM_Hexagon.SM_Hexagon" :!type "StaticMesh Object Reference")))

(event `Shape Pressed`
  (if (not (`TimelineComponent.IsPlaying` (`self.Shape Pressed Timeline`)))
    (`FMODBlueprintStatics.PlayEventAtLocation` "/Game/FMOD/Events/In-Game/Object_Pressed.Object_Pressed" (`KismetMathLibrary.MakeTransform` (`self.K2_GetActorLocation`)))
    (`LegacyCameraShake.StartLegacyCameraShake` (`GameplayStatics.GetPlayerCameraManager` 0) "/Game/Instructions_Tasks/BP_Object_Pressed_CS.BP_Object_Pressed_CS_C" 1.5)
    (bind (_direction _alpha) (`Timeline|Shape Pressed Timeline` :!via `PlayFromStart`)
      (:`Update`
        (`SceneComponent.K2_SetRelativeLocation` (`self.Shape SM`) (`KismetMathLibrary.VLerp` (0.0 0.0 0.0) (0.0 0.0 -10.0) _alpha) false false))
      (:`Finished`
        (`/Game/Instructions_Tasks/Shapes/BP_Shape_Instruction.Shape Child Pressed` (`self.As BP Shape Instruction`) self)))))

(event `Deactivate_Outline_1`
  (`MeshComponent.SetOverlayMaterial` (`self.Shape SM`) null))

(event `Activate_Outline_1`
  (`MeshComponent.SetOverlayMaterial` (`self.Shape SM`) "/Game/Assets/M_Outline.M_Outline"))

(fn `UserConstructionScript`
  (bind _shape_sm (`self.Shape SM`))
  (`StaticMeshComponent.SetStaticMesh` _shape_sm (select `/Game/Instructions_Tasks/Shapes/Enum_Shapes` (`self.Shape Value`) :`NewEnumerator0` "/Game/Assets/Interactions/SM_Diamond.SM_Diamond" :`NewEnumerator1` "/Game/Assets/Interactions/SM_Triangle.SM_Triangle" :`NewEnumerator2` "/Game/Assets/Interactions/SM_Circle.SM_Circle" :`NewEnumerator3` "/Game/Assets/Interactions/SM_Pentagon.SM_Pentagon" :`NewEnumerator4` "/Game/Assets/Interactions/SM_Hexagon.SM_Hexagon" :!type "StaticMesh Object Reference"))
  (`PrimitiveComponent.SetMaterial` _shape_sm 0 "/AnimationSharing/AnimSharingBase.AnimSharingBase"))