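; BP_Shape_Instruction is a shape-matching task in the instruction system, where the player must press the correct one of five child shape actors.
; Setup and enable turn collision on for all five shapes, and a press turns it off on all of them.
; The pressed shape's value is compared to the instruction's correct shape, reporting success or failure through InstructionInteract.
; A wrong press also plays an incorrect-match sound and costs the player a life.
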(event `Shape Child Pressed`
  (params (`Shape Child Ref` :type "/Game/Instructions_Tasks/Shapes/BP_Shape_Child Object Reference"))
  (for _index (range 5)
    (bind _asbp_shape_child (cast `/Game/Instructions_Tasks/Shapes/BP_Shape_Child` (`ChildActorComponent.ChildActor` (select `int` _index :`0` (`self.Shape Child 1`) :`1` (`self.Shape Child 2`) :`2` (`self.Shape Child 3`) :`3` (`self.Shape Child 4`) :`4` (`self.Shape Child 5`)))))
    (`self.SetActorEnableCollision` _asbp_shape_child false))
  (if (`|EnumEquality` (`/Game/Instructions_Tasks/Shapes/BP_Shape_Child.Shape Value` `Shape Child Ref`) (`.CorrectShape_2_C31E352C43B622DE4F851E85862E8FDF` (break `/Game/Instructions_Tasks/Shapes/Struct_Shape_Instruction_Info` (`.ShapesInstructionInfo_25_A4D514E649F730A2E91C87BFACD64FA4` (break `/Game/Instructions_Tasks/Struct_Instruction_Info` (`self.Instruction Info`))))))
    (`self.Instruction Interact` true)
    (else
      (`FMODBlueprintStatics.PlayEventAtLocation` "/Game/FMOD/Events/In-Game/Match_Incorrect.Match_Incorrect" (`KismetMathLibrary.MakeTransform` (`self.K2_GetActorLocation`)))
      (bind _asbp_player (cast `/Game/Player/Blueprints/BP_Player` (`GameplayStatics.GetPlayerCharacter` 0)))
      (`/Game/Player/Blueprints/BP_Player.Decrease Life` _asbp_player)
      (`self.Instruction Interact` false))))

(fn `Complete Instruction`
  (params (Successful :type Boolean))
  (`parent.Complete Instruction` Successful)
  (set `self.Shape Being Pressed` false))

(fn `Enable Instruction`
  (`parent.Enable Instruction`)
  (for _index (range 5)
    (bind _asbp_shape_child (cast `/Game/Instructions_Tasks/Shapes/BP_Shape_Child` (`ChildActorComponent.ChildActor` (select `int` _index :`0` (`self.Shape Child 1`) :`1` (`self.Shape Child 2`) :`2` (`self.Shape Child 3`) :`3` (`self.Shape Child 4`) :`4` (`self.Shape Child 5`)))))
    (`self.SetActorEnableCollision` _asbp_shape_child true)))

(fn `Setup Instruction`
  (params (`Instruction Info` :type "/Game/Instructions_Tasks/Struct_Instruction_Info Structure"))
  (`parent.Setup Instruction` `Instruction Info`)
  (for _index (range 5)
    (bind _asbp_shape_child (cast `/Game/Instructions_Tasks/Shapes/BP_Shape_Child` (`ChildActorComponent.ChildActor` (select `int` _index :`0` (`self.Shape Child 1`) :`1` (`self.Shape Child 2`) :`2` (`self.Shape Child 3`) :`3` (`self.Shape Child 4`) :`4` (`self.Shape Child 5`)))))
    (`self.SetActorEnableCollision` _asbp_shape_child true)))

(fn `UserConstructionScript`
  (`parent.UserConstructionScript`))