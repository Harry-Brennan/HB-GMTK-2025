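; Game instance that holds and persists per-map progress and volume levels through a BP_Save_Game object.
; Load reads the save slot or builds default map entries and volumes, while Save packs both into one struct and writes it.
; UpdateMapInfo matches by map name, keeps completion and the higher score and instruction progress, then saves.
; UpdateVolumeLevels only changes the in-memory values, and getters expose the stored data.
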(event `/Game/Saving_Loading/BPI_Game_Instance.Load`
  (bind _returnvalue (`GameplayStatics.LoadGameFromSlot` "SaveSlot"))
  (`/Engine/EditorBlueprintResources/StandardMacros.IsValid` _returnvalue
    (:`Is Valid`
      (`KismetSystemLibrary.PrintString` "SAVE GAME VALID")
      (bind _asbp_save_game (cast `/Game/Saving_Loading/BP_Save_Game` _returnvalue))
      (bind _output_get (set `self.Game Save Data` (`/Game/Saving_Loading/BP_Save_Game.Save Info` _asbp_save_game)))
      (bind (_mapinfo _volumelevels) (break `/Game/Saving_Loading/Struct_Save_Info` _output_get))
      (set `self.Maps Info` _mapinfo)
      (set `self.Volume Levels` _volumelevels))
    (:`Is Not Valid`
      (`KismetSystemLibrary.PrintString` "SAVE GAME NOT VALID")
      (set `self.Maps Info` (`|MakeArray` (make `/Game/Maps/Struct_Map_Info` "NewEnumerator0") (make `/Game/Maps/Struct_Map_Info` "NewEnumerator1") (make `/Game/Maps/Struct_Map_Info` "NewEnumerator2") (make `/Game/Maps/Struct_Map_Info` "NewEnumerator3") (make `/Game/Maps/Struct_Map_Info` "NewEnumerator4")))
      (set `self.Volume Levels` (`|MakeArray` 0.75 0.75 0.75)))))

(event `/Game/Saving_Loading/BPI_Game_Instance.Save`
  (bind _created_save_game (`self.Created Save Game`))
  (`self.Created Save Game`
    (:`then`
      _)
    (:`else`
      (bind _returnvalue (`GameplayStatics.CreateSaveGameObject` "/Game/Saving_Loading/BP_Save_Game.BP_Save_Game_C"))
      (set `self.Created Save Game` _returnvalue)))
  (set `self.Game Save Data` (make `/Game/Saving_Loading/Struct_Save_Info` (`self.Maps Info`) (`self.Volume Levels`)))
  (set `/Game/Saving_Loading/BP_Save_Game.Save Info` (`self.Game Save Data`) _created_save_game)
  (`GameplayStatics.SaveGameToSlot` (`self.Created Save Game`) (`/Game/Saving_Loading/BP_Save_Game.Slot Name` _created_save_game) (`/Game/Saving_Loading/BP_Save_Game.User Index` _created_save_game)))

(event `/Game/Saving_Loading/BPI_Game_Instance.Update Map Info`
  (params (`New Map Info` :type "/Game/Maps/Struct_Map_Info Structure"))
  (bind (_mapname _completed _savedscore _instructionscomplete) (break `/Game/Maps/Struct_Map_Info` `New Map Info`))
  (bind (_mapname_2 _completed_2 _savedscore_2 _instructionscomplete_2) (break `/Game/Maps/Struct_Map_Info` (`|GetArrayItem` (`self.Maps Info`) (`self.Map Info Index To Update`))))
  (for (_array_element _array_index) (`self.Maps Info`)
    (if (`|EnumEquality` (`.MapName_3_09593CA946836AEED176C5A0B5DF109F` (break `/Game/Maps/Struct_Map_Info` `New Map Info`)) (`.MapName_3_09593CA946836AEED176C5A0B5DF109F` (break `/Game/Maps/Struct_Map_Info` _array_element)))
      (set `self.Map Info Index To Update` _array_index)
      (break)))
  (`KismetArrayLibrary.Array_Set` (`self.Maps Info`) (`self.Map Info Index To Update`) (make `/Game/Maps/Struct_Map_Info` _mapname (select `bool` _completed_2 :`false` _completed :`true` _completed_2) (`KismetMathLibrary.SelectInt` _savedscore_2 _savedscore (> _savedscore_2 _savedscore)) (`KismetMathLibrary.SelectInt` _instructionscomplete_2 _instructionscomplete (> _instructionscomplete_2 _instructionscomplete))))
  (`self.Save`))

(event `/Game/Saving_Loading/BPI_Game_Instance.Update Volume Levels`
  (params (`New Volume Levels` :type "Array of Float (double-precision) (by ref)"))
  (set `self.Volume Levels` `New Volume Levels`))

(fn `Get Map Info`
  (returns (`Map Info` :type "Array of /Game/Maps/Struct_Map_Info Structure"))
  (return (`self.Maps Info`)))

(fn `Get Saved Info`
  (returns (`Save Data` :type "/Game/Saving_Loading/Struct_Save_Info Structure"))
  (return (`self.Game Save Data`)))

(fn `Get Volume Levels`
  (returns (`Volume Levels` :type "Array of Float (double-precision)"))
  (return (`self.Volume Levels`)))